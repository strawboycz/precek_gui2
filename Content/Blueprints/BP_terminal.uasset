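; BP_terminal is a terminal actor that shows an interact prompt widget while the player character overlaps it.
; Begin overlap creates a UW_interact widget, stores it and adds it to the viewport, and end overlap removes it from its parent.
; StopWidgets sets a flag that blocks new prompts and removes the current one, while ResumeWidgets clears that flag.
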(event EventBeginPlay)

(event Collision|EventActorBeginOverlap
  (params (OtherActor :type Actor%20Object%20Reference))
  (if (not (Variables|Default|GetStop_widgets))
    (if (== OtherActor (Game|GetPlayerCharacter 0))
      (CallFunction|ShowInteractWidget))))

(event EventTick
  (params (DeltaSeconds :type Float%20%28single-precision%29)))

(event Collision|EventActorEndOverlap
  (params (OtherActor :type Actor%20Object%20Reference))
  (if (== (Game|GetPlayerCharacter 0) OtherActor)
    (CallFunction|DestroyInteractWidget)))

(fn ConstructionScript)

(fn ShowInteractWidget
  (bind _returnvalue (UserInterface|CreateWidget "/Game/Widgets/UW_interact.UW_interact_C"))
  (Variables|Default|SetinteractWidget _returnvalue)
  (UserInterface|Viewport|AddtoViewport _returnvalue 0))

(fn DestroyInteractWidget
  (Widget|RemovefromParent (Variables|Default|GetinteractWidget)))

(fn StopWidgets
  (Variables|Default|SetStop_widgets true)
  (CallFunction|DestroyInteractWidget))

(fn ResumeWidgets
  (Variables|Default|SetStop_widgets false))