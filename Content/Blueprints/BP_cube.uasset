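; BP_cube is an actor with a cube that can spin around its vertical axis and be resized.
; While ShouldSpin is set, Tick adds a yaw step scaled by RotCoeficient, without delta time, so speed depends on frame rate.
; BeginPlay caches the starting world scale, and ChangeSize offsets that cached scale by the given value, so repeated calls do not accumulate.
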(event EventBeginPlay
  (Variables|Default|Setdefault%20scale (Transformation|GetWorldScale (Variables|Default|GetCube))))

(event Collision|EventActorBeginOverlap
  (params (OtherActor :type Actor%20Object%20Reference)))

(event EventTick
  (params (DeltaSeconds :type Float%20%28single-precision%29))
  (bind _cube (Variables|Default|GetCube))
  (bind _returnvalue (Transformation|GetWorldRotation _cube))
  (bind (_roll _pitch _yaw) (Math|Rotator|BreakRotator _returnvalue))
  (if (Variables|Default|GetShouldSpin)
    (Transformation|SetWorldRotation _cube (Math|Rotator|MakeRotator _roll _pitch (+ _yaw (* 0.1 (Variables|Default|GetRotCoeficient)))) false false)))

(fn ConstructionScript)

(fn ChangeSize
  (params (value :type Vector))
  (Transformation|SetWorldScale3D (Variables|Default|GetCube) (+ value (Variables|Default|Getdefault%20scale))))